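; NormalMonster_BP is a normal monster Blueprint whose graph plays a dissolve effect when the monster dies.
; MonsterIsDead creates dynamic materials for the skeleton mesh and weapon mesh, then gives them and the PDissolveEdge Niagara system a shared texture.
; A timeline lerps Amount from one to zero on materials and particles together, keeping the dissolve edge in sync.
; The edge width is set at the start and zeroed when the timeline finishes.
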(event `self.ReceiveBeginPlay`)

(event `MonsterIsDead`
  (bind _texture (`self.Texture`))
  (bind _p_dissolveedge (`self.P_DissolveEdge`))
  (`NiagaraComponent.SetVariableFloat` (`self.P_DissolveEdge`) "User.Width" 0.1)
  ;[1 1 1] 캐릭터 스켈레탈메쉬가 들고있는 Material 0, 1, 2
  (bind _returnvalue (`PrimitiveComponent.CreateDynamicMaterialInstance` (`self.Mesh`) 0 "/Game/SKnight_modular/Skeleton/materials/MI_Skeleton_Inst.MI_Skeleton_Inst" "None"))
  ;[1 1 1] 스켈레탈메쉬 검, 방패
  (bind _returnvalue_2 (`PrimitiveComponent.CreateDynamicMaterialInstance` (`self.SK_weapon_01`) 0 "/Game/SKnight_modular/Skeleton_Knight_01/materials/MatInst/MI_weapon_01_Inst.MI_weapon_01_Inst" "None"))
  (`MaterialInstanceDynamic.SetTextureParameterValue` _returnvalue "Texture" _texture)
  (`MaterialInstanceDynamic.SetTextureParameterValue` null "Texture" _texture)
  (`MaterialInstanceDynamic.SetTextureParameterValue` null "Texture" _texture)
  (`MaterialInstanceDynamic.SetTextureParameterValue` _returnvalue_2 "Texture" _texture)
  (`NiagaraFunctionLibrary.SetTextureObject` (`self.P_DissolveEdge`) "Texture" _texture)
  (bind (_direction _time) (`Timeline|타임라인` :!via `PlayFromStart`)
    (:`Update`
      (`MaterialInstanceDynamic.SetScalarParameterValue` _returnvalue "Amount" (`KismetMathLibrary.Lerp` 1.0 0.0 _time))
      (`MaterialInstanceDynamic.SetScalarParameterValue` _returnvalue_2 "Amount" (`KismetMathLibrary.Lerp` 1.0 0.0 _time))
      (`MaterialInstanceDynamic.SetScalarParameterValue` null "Amount" (`KismetMathLibrary.Lerp` 1.0 0.0 _time))
      (`MaterialInstanceDynamic.SetScalarParameterValue` null "Amount" (`KismetMathLibrary.Lerp` 1.0 0.0 _time))
      (`NiagaraComponent.SetVariableFloat` _p_dissolveedge "User.Amount" (`KismetMathLibrary.Lerp` 1.0 0.0 _time)))
    (:`Finished`
      (`NiagaraComponent.SetVariableFloat` _p_dissolveedge "User.Width" 0.0))))

(fn `UserConstructionScript`)